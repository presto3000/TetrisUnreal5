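; Falling tetromino piece for a Tetris-style game that descends on a grid and locks in place when it lands.
; The construction script randomly arranges four cubes into one of seven shapes and tints their glow material.
; A looping timer traces below each cube for WorldStatic, stepping the actor down if clear.
; Otherwise it spawns colored B_SingleBlock actors at each cube, spawns the next B_FallingBlock, and destroys itself.
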(event `self.ReceiveBeginPlay`
  (bind _returnvalue (`KismetSystemLibrary.K2_SetTimerDelegate` (delegate `DropBlock`) (`self.DropSpeed`) true))
  (set `self.BlockDroppingTime` _returnvalue))

(event `DropBlock`
  (set `self.bShouldDrop` true)
  (for _array_element (`SceneComponent.GetChildrenComponents` (`self.DefaultSceneRoot`) false)
    (bind _returnvalue (`SceneComponent.K2_GetComponentLocation` _array_element))
    (bind (_outhit _returnvalue_2) (`KismetSystemLibrary.LineTraceSingleForObjects` _returnvalue (- _returnvalue (0.0 0.0 50.0)) (`|MakeArray` "ObjectTypeQuery1" :!type "EObjectTypeQuery Enum")))
    (if _returnvalue_2
      (`/Engine/EditorBlueprintResources/StandardMacros.DoOnce` false
        (:`Completed`
          (set `self.bShouldDrop` false)
          (`KismetSystemLibrary.K2_ClearAndInvalidateTimerHandle` (`self.BlockDroppingTime`))))))
  (if (`self.bShouldDrop`)
    (`self.K2_AddActorLocalOffset` (0.0 0.0 -50.0))
    (else
      (for _array_element_2 (`SceneComponent.GetChildrenComponents` (`self.DefaultSceneRoot`) false)
        (`|SpawnActorFromClass` "/Game/BLUEPRINTS/B_SingleBlock.B_SingleBlock_C" (`KismetMathLibrary.MakeTransform` (`SceneComponent.K2_GetComponentLocation` _array_element_2)) "Undefined" "OverrideRootScale" null (`self.BlockColor`) null))
      (`|SpawnActorFromClass` "B_FallingBlock_C" (`KismetMathLibrary.MakeTransform` (0.0 0.0 1000.0)) "Undefined" "OverrideRootScale" null null)
      (`self.K2_DestroyActor`))))

(fn `UserConstructionScript`
  (switch `int` (`KismetMathLibrary.RandomIntegerInRange` 0 6)
    (:`0`
      ;[1 1 1] MAKE LINE BLOCK
      (`SceneComponent.K2_AddLocalOffset` (`self.Cube2`) (0.0 0.0 50.0) false false)
      (`SceneComponent.K2_AddLocalOffset` (`self.Cube3`) (0.0 0.0 100.0) false false)
      (`SceneComponent.K2_AddLocalOffset` (`self.Cube4`) (0.0 0.0 150.0) false false)
      (set `self.BlockColor` (struct :`R` 0.999446 :`G` 1.0 :`A` 1.0)))
    (:`1`
      ;[1 1 1] MAKE L BLOCK
      (`SceneComponent.K2_AddLocalOffset` (`self.Cube2`) (0.0 0.0 50.0) false false)
      (`SceneComponent.K2_AddLocalOffset` (`self.Cube3`) (0.0 0.0 100.0) false false)
      (`SceneComponent.K2_AddLocalOffset` (`self.Cube4`) (0.0 50.0 0.0) false false)
      (set `self.BlockColor` (struct :`R` 1.0 :`B` 0.016021 :`A` 1.0)))
    (:`2`
      ;[1 1 1] MAKE REVERSE L BLOCK
      (`SceneComponent.K2_AddLocalOffset` (`self.Cube2`) (0.0 0.0 50.0) false false)
      (`SceneComponent.K2_AddLocalOffset` (`self.Cube3`) (0.0 0.0 100.0) false false)
      (`SceneComponent.K2_AddLocalOffset` (`self.Cube4`) (0.0 -50.0 0.0) false false)
      (set `self.BlockColor` (struct :`R` 1.0 :`G` 0.39094 :`A` 1.0)))
    (:`3`
      ;[1 1 1] MAKE S BLOCK
      (`SceneComponent.K2_AddLocalOffset` (`self.Cube2`) (0.0 0.0 50.0) false false)
      (`SceneComponent.K2_AddLocalOffset` (`self.Cube3`) (0.0 50.0 50.0) false false)
      (`SceneComponent.K2_AddLocalOffset` (`self.Cube4`) (0.0 50.0 100.0) false false)
      (set `self.BlockColor` (struct :`R` 1.0 :`G` 0.017876 :`B` 0.869642 :`A` 1.0)))
    (:`4`
      ;[1 1 1] MAKE REVERSE S BLOCK
      (`SceneComponent.K2_AddLocalOffset` (`self.Cube2`) (0.0 0.0 50.0) false false)
      (`SceneComponent.K2_AddLocalOffset` (`self.Cube3`) (0.0 -50.0 50.0) false false)
      (`SceneComponent.K2_AddLocalOffset` (`self.Cube4`) (0.0 -50.0 100.0) false false)
      (set `self.BlockColor` (struct :`G` 0.005852 :`B` 1.0 :`A` 1.0)))
    (:`5`
      ;[1 1 1] MAKE T BLOCK
      (`SceneComponent.K2_AddLocalOffset` (`self.Cube2`) (0.0 -50.0 0.0) false false)
      (`SceneComponent.K2_AddLocalOffset` (`self.Cube3`) (0.0 50.0 0.0) false false)
      (`SceneComponent.K2_AddLocalOffset` (`self.Cube4`) (0.0 0.0 50.0) false false)
      (set `self.BlockColor` (struct :`G` 0.816944 :`B` 1.0 :`A` 1.0)))
    (:`6`
      ;[1 1 1] MAKE SQUARE BLOCK
      (`SceneComponent.K2_AddLocalOffset` (`self.Cube2`) (0.0 0.0 50.0) false false)
      (`SceneComponent.K2_AddLocalOffset` (`self.Cube3`) (0.0 50.0 0.0) false false)
      (`SceneComponent.K2_AddLocalOffset` (`self.Cube4`) (0.0 50.0 50.0) false false)
      (set `self.BlockColor` (struct :`G` 1.0 :`B` 0.045393 :`A` 1.0))))
  (`MeshComponent.SetVectorParameterValueOnMaterials` (`self.Cube1`) "GlowColor" (`KismetMathLibrary.Conv_LinearColorToVector` (`self.BlockColor`)))
  (`MeshComponent.SetVectorParameterValueOnMaterials` (`self.Cube2`) "GlowColor" (`KismetMathLibrary.Conv_LinearColorToVector` (`self.BlockColor`)))
  (`MeshComponent.SetVectorParameterValueOnMaterials` (`self.Cube3`) "GlowColor" (`KismetMathLibrary.Conv_LinearColorToVector` (`self.BlockColor`)))
  (`MeshComponent.SetVectorParameterValueOnMaterials` (`self.Cube4`) "GlowColor" (`KismetMathLibrary.Conv_LinearColorToVector` (`self.BlockColor`))))