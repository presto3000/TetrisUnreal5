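; Actor that detects and clears completed lines of B_SingleBlock actors in a falling-block, Tetris-style game.
; CheckLines treats each BoxComponent as a row sensor, counting a row full at ten overlapping blocks and increasing DropAmount.
; A full row below CutoffLineZ lowers that cutoff and has its blocks exploded and destroyed.
; Finally, every block above the cutoff has its TargetZ lowered by DropAmount, neither value being reset here.
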(fn `CheckLines`
  (locals (DropAmount :type "Float (double-precision)") (OverlappingActors :type "Array of Actor Object Reference") (CutoffLineZ :type "Float (double-precision)" :default 2000.0))
  (for _array_element (`self.K2_GetComponentsByClass` "/Script/Engine.BoxComponent")
    (set `local.OverlappingActors` (`PrimitiveComponent.GetOverlappingActors` _array_element "/Game/BLUEPRINTS/B_SingleBlock.B_SingleBlock_C"))
    (if (== (`KismetArrayLibrary.Array_Length` (`local.OverlappingActors`)) 10)
      (set `local.DropAmount` (+ (`local.DropAmount`) 50.0))
      (bind (_returnvalue_x _returnvalue_y _returnvalue_z) (`KismetMathLibrary.BreakVector` (`SceneComponent.K2_GetComponentLocation` _array_element)))
      (if (< _returnvalue_z (`local.CutoffLineZ`))
        (set `local.CutoffLineZ` _returnvalue_z)
        (for _array_element_2 (`local.OverlappingActors`)
          (`GameplayStatics.SpawnEmitterAtLocation` "/Game/StarterContent/Particles/P_Explosion.P_Explosion" (`self.K2_GetActorLocation` _array_element_2) (struct) (0.5 0.5 0.5))
          (`self.K2_DestroyActor` _array_element_2)))))
  (bind _outactors (`GameplayStatics.GetAllActorsOfClass` "/Game/BLUEPRINTS/B_SingleBlock.B_SingleBlock_C"))
  (for _array_element_3 _outactors
    (bind (_returnvalue_x_2 _returnvalue_y_2 _returnvalue_z_2) (`KismetMathLibrary.BreakVector` (`self.K2_GetActorLocation` _array_element_3)))
    (if (> _returnvalue_z_2 (`local.CutoffLineZ`))
      (set `/Game/BLUEPRINTS/B_SingleBlock.TargetZ` (- (`/Game/BLUEPRINTS/B_SingleBlock.TargetZ` _array_element_3) (`local.DropAmount`)) _array_element_3))))

(fn `UserConstructionScript`)